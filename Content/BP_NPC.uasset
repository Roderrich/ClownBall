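; NPC Blueprint that reacts to the player ball with a single AI move, apparently intended as running away.
; Tick checks the distance from its cube to the ball found at BeginPlay and, within range, issues AIMoveTo with debug prints.
; The destination is the raw ball-minus-cube XY offset at the ball's height, and HasDestination never resets.
; ChaseCharacter has no target and MoveToRandom is an empty stub.
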(event Custom|MoveToRandom)

(event Custom|Chase%20Character
  (AI|AIMoveTo self "0, 0, 0" 0 5.0 false))

(event EventBeginPlay
  (bind _returnvalue (Actor|GetActorOfClass "/Game/BP_PlayerBall.BP_PlayerBall_C"))
  (Variables|Default|SetPlayerVar _returnvalue))

(event EventTick
  (params (DeltaSeconds :type Float%20%28single-precision%29))
  (bind _playervar (Variables|Default|GetPlayerVar))
  (bind _cube (Variables|Default|GetCube))
  (bind _returnvalue (Transformation|GetWorldLocation _cube))
  (bind _sm_ball (Variables|/Game/BP_PlayerBall.BP_PlayerBall_C|GetSM_Ball _playervar))
  (bind (_x _y) (Class|KismetMathLibrary|BreakVector3f _returnvalue))
  (bind _returnvalue_2 (Transformation|GetWorldLocation _sm_ball))
  (bind (_x_2 _y_2 _z) (Class|KismetMathLibrary|BreakVector3f _returnvalue_2))
  (bind _returnvalue_3 (- _x_2 _x))
  (bind _returnvalue_4 (- _y_2 _y))
  (bind _returnvalue_5 (Math|Vector|MakeVector _returnvalue_3 _returnvalue_4 _z))
  (if (<= (Math|Vector|Distance(Vector) _returnvalue_2 _returnvalue) 5e+02)
    (if (not (stale _output_get))
      (Development|PrintString "Tried running")
      (bind _output_get (Variables|Default|Sethas%20destination true))
      (Development|PrintString (Utilities|String|ToString(Float) (Math|Vector|VectorLengthXY _returnvalue_5)))
      (AI|AIMoveTo self _returnvalue_5 0 5.0 false
        (:OnSuccess
          (Development|PrintString "Made it"))))))

(fn ConstructionScript)