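; BP_KickableLady is a physics prop that gets knocked away when the player ball hits it.
; On a component hit from BP_PlayerBall, it applies a velocity-change impulse at the impact point.
; The impulse adds an upward boost to the hit's normal impulse and divides the sum by a damping float, AntiBonkFloat.
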(event OnComponentHit(SM_KickLady)
  (params (HitComponent :type Primitive%20Component%20Object%20Reference) (OtherActor :type Actor%20Object%20Reference) (OtherComp :type Primitive%20Component%20Object%20Reference) (NormalImpulse :type Vector :default "0, 0, 0") (Hit :type Hit%20Result%20Structure%20%28by%20ref%29))
  (Utilities|Casting|CastToBP_PlayerBall OtherActor)
  (Class|PrimitiveComponent|AddVelocityChangeImpulseatLocation (Variables|Default|GetSM_KickLady) (* (/ (+ NormalImpulse (* (Math|Vector|VectorUp) (Variables|Default|GetUpness))) (Variables|Default|GetAntiBonkFloat)) (Variables|Default|Get1)) (.ImpactPoint (Collision|BreakHitResult Hit)) "None"))

(fn ConstructionScript)