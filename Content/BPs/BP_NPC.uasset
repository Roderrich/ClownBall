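; BP_NPC is an AI character that flees the player ball and gets knocked flying when the ball hits it.
; Each Tick, while the ball is within 500 units of its Cube, it compares X and Y positions and calls AIMoveTo toward a diagonal point away from the ball, offset by Speed.
; When the ball overlaps the Cube, the capsule enables physics and receives an up-and-forward impulse scaled by Strength.
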(event OnComponentBeginOverlap(Cube)
  (params (OverlappedComponent :type Primitive%20Component%20Object%20Reference) (OtherActor :type Actor%20Object%20Reference) (OtherComp :type Primitive%20Component%20Object%20Reference) (OtherBodyIndex :type Integer) (bFromSweep :type Boolean) (SweepResult :type Hit%20Result%20Structure%20%28by%20ref%29))
  (bind _capsulecomponent (Variables|Collision|GetCapsuleComponent))
  (Utilities|Casting|CastToBP_PlayerBall OtherActor)
  (Physics|SetSimulatePhysics _capsulecomponent true)
  (Class|PrimitiveComponent|AddVelocityChangeImpulseatLocation _capsulecomponent (* (+ (Math|Vector|GetUpVector _capsulecomponent) (Math|Vector|GetForwardVector _capsulecomponent)) (Variables|Default|GetStrength)) "0, 0, 0" "None"))

(event EventBeginPlay
  (bind _returnvalue (Actor|GetActorOfClass "/Game/BPs/BP_PlayerBall.BP_PlayerBall_C"))
  (Variables|Default|SetPlayerVar _returnvalue))

(event EventTick
  (params (DeltaSeconds :type Float%20%28single-precision%29))
  (bind _playervar (Variables|Default|GetPlayerVar))
  (bind _speed (Variables|Default|GetSpeed))
  (bind _cube (Variables|Default|GetCube))
  (bind _returnvalue (Transformation|GetWorldLocation _cube))
  (bind _sm_ball (Variables|/Game/BPs/BP_PlayerBall.BP_PlayerBall_C|GetSM_Ball _playervar))
  (bind (_x _y) (Class|KismetMathLibrary|BreakVector3f _returnvalue))
  (bind _returnvalue_2 (Transformation|GetWorldLocation _sm_ball))
  (bind (_x_2 _y_2) (Class|KismetMathLibrary|BreakVector3f _returnvalue_2))
  (bind _returnvalue_3 (< _y_2 _y))
  (if (<= (Math|Vector|Distance(Vector) _returnvalue_2 _returnvalue) 5e+02)
    (if (< _x_2 _x)
      (if _returnvalue_3
        (AI|AIMoveTo self (+ (* (+ (Class|KismetMathLibrary|VectorRight) (Class|KismetMathLibrary|VectorForward)) _speed) _returnvalue) 0 0.5 false)
        (else
          (AI|AIMoveTo self (+ (* (+ (Class|KismetMathLibrary|VectorLeft) (Class|KismetMathLibrary|VectorForward)) _speed) _returnvalue) 0 0.5 false)))
      (elif _returnvalue_3
        (AI|AIMoveTo self (+ (* (+ (Class|KismetMathLibrary|VectorRight) (Class|KismetMathLibrary|VectorBackward)) _speed) _returnvalue) 0 0.5 false)
        (else
          (AI|AIMoveTo self (+ (* (+ (Class|KismetMathLibrary|VectorLeft) (Class|KismetMathLibrary|VectorBackward)) _speed) _returnvalue) 0 0.5 false))))))

(fn ConstructionScript)