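; BP_Roullette is a roulette table actor that spins its mesh around the yaw axis in a continuous speed-up and slow-down cycle.
; A looping timer starts on BeginPlay and calls RotateTable about 60 times a second, adding a world rotation scaled by SpeedRot.
; FloatBaseMove ramps linearly between zero and one by SpeeddChange per tick, with ShouldSpeedUP flipping at each end.
; The delayed restart branch never runs here, since nothing clears ShouldRotate.
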(event Custom|RotateTable
  (bind _sm_roullette (Variables|Default|GetSM_Roullette))
  (if (Variables|Default|GetShouldRotate)
    (if (Variables|Default|GetShouldSpeedUP)
      (Transformation|AddWorldRotation _sm_roullette (Math|Rotator|MakeRotator 0.0 0.0 (* (Variables|Default|GetFloatBaseMove) (Variables|Default|GetSpeedRot))) false false)
      (if (< (Variables|Default|GetFloatBaseMove) 1.0)
        (Variables|Default|SetFloatBaseMove (+ (Variables|Default|GetFloatBaseMove) (Variables|Default|GetSpeeddChange)))
        (else
          (Variables|Default|SetShouldSpeedUP false)))
      (else
        (Transformation|AddWorldRotation _sm_roullette (Math|Rotator|MakeRotator 0.0 0.0 (* (Variables|Default|GetFloatBaseMove) (Variables|Default|GetSpeedRot))) false false)
        (if (> (Variables|Default|GetFloatBaseMove) 0.0)
          (Variables|Default|SetFloatBaseMove (- (Variables|Default|GetFloatBaseMove) (Variables|Default|GetSpeeddChange)))
          (else
            (Variables|Default|SetShouldRotate true)
            (Variables|Default|SetShouldSpeedUP true)))))
    (else
      (Utilities|FlowControl|Delay (Variables|Default|GetInitial%20Start%20Delay))
      (Variables|Default|SetShouldRotate true)
      (Variables|Default|SetShouldSpeedUP false))))

(event EventBeginPlay
  (Utilities|Time|SetTimerbyEvent (delegate Custom|RotateTable) 0.016667 true (Variables|Default|GetInitial%20Start%20Delay))
  (Variables|Default|SetShouldRotate true)
  (Variables|Default|SetShouldSpeedUP true))

(fn ConstructionScript)