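; BP_NPC1 is an NPC pawn that periodically chases the player ball and attempts a one-time evasive move when it comes close.
; A looping timer issues AI MoveTo toward the BP_PlayerBall found at BeginPlay.
; Tick watches ball-to-Cube distance and, once within range, sets HasDestination, never reset, and moves to their raw XY difference as a world position.
; RunAwayCharacter and MoveToRandom are empty stubs.
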(event Custom|MoveToRandom)

(event Custom|Chase%20Character
  (AI|AIMoveTo self "0, 0, 0" (Variables|Default|GetPlayerVar) 0.5 false))

(event Custom|Run%20Away%20Character)

(event EventBeginPlay
  (bind _returnvalue (Actor|GetActorOfClass "/Game/BPs/BP_PlayerBall.BP_PlayerBall_C"))
  (Variables|Default|SetPlayerVar _returnvalue)
  (Utilities|Time|SetTimerbyEvent (delegate Custom|Chase%20Character) 5.0 true 5.0))

(event EventTick
  (params (DeltaSeconds :type Float%20%28single-precision%29))
  (bind _self self)
  (bind _playervar (Variables|Default|GetPlayerVar))
  (bind _sm_ball (Variables|/Game/BPs/BP_PlayerBall.BP_PlayerBall_C|GetSM_Ball _playervar))
  (bind _cube (Variables|Default|GetCube _self))
  (bind _returnvalue (Transformation|GetWorldLocation _sm_ball))
  (bind _returnvalue_2 (Transformation|GetWorldLocation _cube))
  (bind (_x _y _z) (Class|KismetMathLibrary|BreakVector3f _returnvalue))
  (bind (_x_2 _y_2) (Class|KismetMathLibrary|BreakVector3f _returnvalue_2))
  (bind _returnvalue_3 (- _x _x_2))
  (bind _returnvalue_4 (- _y _y_2))
  (bind _returnvalue_5 (Math|Vector|MakeVector _returnvalue_3 _returnvalue_4 _z))
  (if (<= (Math|Vector|Distance(Vector) _returnvalue _returnvalue_2) 5e+02)
    (if (not (stale _output_get))
      (Development|PrintString "Tried running")
      (bind _output_get (Variables|Default|Sethas%20destination true))
      (Development|PrintString (Utilities|String|ToString(Float) (Math|Vector|VectorLengthXY _returnvalue_5)))
      (AI|AIMoveTo self _returnvalue_5 0 5.0 false
        (:OnSuccess
          (Development|PrintString "Made it"))))))

(fn ConstructionScript)